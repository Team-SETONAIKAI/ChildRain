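; A slippery slope gimmick that makes the player character slide while inside its Box坂 trigger volume.
; On begin overlap by player pawn 0, it zeroes the CharacterMovement ground friction and walking braking deceleration.
; On end overlap, it writes back hardcoded normal values rather than the character's previous settings, with debug prints on both events.
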(event `self.Box(坂).OnComponentBeginOverlap`
  (params (OverlappedComponent :type "PrimitiveComponent Object Reference") (OtherActor :type "Actor Object Reference") (OtherComp :type "PrimitiveComponent Object Reference") (OtherBodyIndex :type Integer) (bFromSweep :type Boolean) (SweepResult :type "HitResult Structure (by ref)"))
  (if (== OtherActor (`GameplayStatics.GetPlayerPawn` 0))
    (bind _ascharacter (cast `Character` OtherActor))
    (bind _charactermovement (`Character.CharacterMovement` _ascharacter))
    (set `CharacterMovementComponent.GroundFriction` 0.0 _charactermovement)
    (set `CharacterMovementComponent.BrakingDecelerationWalking` 0.0 _charactermovement)
    (`KismetSystemLibrary.PrintString` "set")))

(event `self.Box(坂).OnComponentEndOverlap`
  (params (OverlappedComponent :type "PrimitiveComponent Object Reference") (OtherActor :type "Actor Object Reference") (OtherComp :type "PrimitiveComponent Object Reference") (OtherBodyIndex :type Integer))
  (if (== OtherActor (`GameplayStatics.GetPlayerPawn` 0))
    (bind _ascharacter (cast `Character` OtherActor))
    (bind _charactermovement (`Character.CharacterMovement` _ascharacter))
    (set `CharacterMovementComponent.GroundFriction` 8.0 _charactermovement)
    (set `CharacterMovementComponent.BrakingDecelerationWalking` 2048.0 _charactermovement)
    (`KismetSystemLibrary.PrintString` "kaizho")))

(fn `UserConstructionScript`)