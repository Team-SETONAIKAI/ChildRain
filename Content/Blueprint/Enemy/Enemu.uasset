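; Enemy Blueprint that senses the player through AI Perception and deals damage with a forward attack.
; Perception updates store the player pawn in SceneActor, clear it after a delay when a stimulus is lost, and GetSensingInfo exposes it.
; The Attack event waits, plays a sound, then box-traces along the forward vector over AttackRange and damages the player on a hit.
; Debug prints show the controller path on BeginPlay and report lost sight.
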(event `self.ReceiveBeginPlay`
  (`parent.ReceiveBeginPlay`)
  (`KismetSystemLibrary.PrintString` (`KismetSystemLibrary.GetPathName` (`self.GetController`)) true true (struct :`G` 0.66 :`B` 1.0 :`A` 1.0) 10.0))

(event `self.ReceiveTick`
  (params (DeltaSeconds :type "Float (single-precision)"))
  (`parent.ReceiveTick` DeltaSeconds))

(event `self.AIPerception.OnPerceptionUpdated`
  (params (UpdatedActors :type "Array of Actor Object Reference (by ref)"))
  (bind _returnvalue (`GameplayStatics.GetPlayerPawn` 0))
  ;[1 1 1] AI Perception
  (for _array_element UpdatedActors
    (bind _info (`AIPerceptionComponent.GetActorsPerception` (`self.AIPerception`) _array_element))
    (bind (_target _lastsensedstimuli) (break `ActorPerceptionBlueprintInfo` _info))
    (if (`.bSuccessfullySensed` (break `AIStimulus` (`|GetArrayItem` _lastsensedstimuli)))
      (if (== _target _returnvalue)
        (set `self.SceneActor` _returnvalue))
      (else
        (`KismetSystemLibrary.Delay` 5.0)
        (set `self.SceneActor` null)
        (`KismetSystemLibrary.PrintString` "見えね…")))))

(event `Attack`
  (params (AttackRange :type "Float (double-precision)"))
  (bind _returnvalue (`self.K2_GetActorLocation`))
  (bind _returnvalue_2 (`GameplayStatics.GetPlayerPawn` 0))
  ;[1 1 1] Attack
  (`KismetSystemLibrary.Delay` 2.0)
  (`GameplayStatics.SpawnSoundAtLocation` "/Game/StarterContent/Audio/Collapse01.Collapse01" (`self.K2_GetActorLocation`) (struct) 1.0 1.0 0.0 null null)
  (bind (_outhit _returnvalue_3) (`KismetSystemLibrary.BoxTraceSingle` :`Start` _returnvalue :`End` (+ _returnvalue (* (`self.GetActorForwardVector`) AttackRange)) :`HalfSize` (30.0 30.0 30.0) :`TraceChannel` "TraceTypeQuery1" :`DrawDebugType` "ForOneFrame"))
  (if _returnvalue_3
    (if (== (`.HitActor` (`GameplayStatics.BreakHitResult` _outhit)) _returnvalue_2)
      (`GameplayStatics.ApplyDamage` _returnvalue_2 5.0))))

(fn `GetSensingInfo`
  (returns (SceneActor :type "Actor Object Reference"))
  (return (`self.SceneActor`)))

(fn `UserConstructionScript`
  (`parent.UserConstructionScript`))