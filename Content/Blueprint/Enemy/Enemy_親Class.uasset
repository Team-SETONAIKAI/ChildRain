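; Parent enemy character class that handles health, hit reaction and death.
; BeginPlay marks it alive if the player pawn is a RainBoy, and Tick caches the frame's delta time.
; Damage reduces health; surviving hits print a cry and launch the enemy horizontally toward the damage causer along the look-at yaw.
; At zero health it clears the alive flag and ragdolls the mesh with physics.
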(event `self.ReceiveBeginPlay`
  (cast `/Game/Blueprint/RainBoy/RainBoy` (`GameplayStatics.GetPlayerPawn` 0))
  (set `self.Alive` true))

(event `self.ReceiveTick`
  (params (DeltaSeconds :type "Float (single-precision)"))
  (set `self.DeltaTime` DeltaSeconds))

(event `self.ReceiveAnyDamage`
  (params (Damage :type "Float (single-precision)") (DamageType :type "DamageType Object Reference") (InstigatedBy :type "Controller Object Reference") (DamageCauser :type "Actor Object Reference"))
  (bind _output_get (set `self.Health` (- (`self.Health`) Damage)))
  (if (<= _output_get 0.0)
    (set `self.Alive` false)
    (`PrimitiveComponent.SetCollisionEnabled` (`self.Mesh`) "QueryAndPhysics")
    (`SkeletalMeshComponent.SetAllBodiesSimulatePhysics` (`self.Mesh`) true)
    (else
      (`KismetSystemLibrary.PrintString` "Enemy「うわぁぁぁ！」")
      (`self.LaunchCharacter` (* (`KismetMathLibrary.GetForwardVector` (`KismetMathLibrary.MakeRotator` 0.0 0.0 (.yaw (`KismetMathLibrary.FindLookAtRotation` (`self.K2_GetActorLocation`) (`self.K2_GetActorLocation` DamageCauser))))) 2000.0) true true))))

(fn `UserConstructionScript`)