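; Imaginary friend actor (イマジナリーフレンド_M2) with an attack that breaks destructible cardboard boxes (段ボール_DM).
; The Img_Attack press enables overlap events on its Box component, which acts as the hit volume.
; An overlapped cardboard box gets physics simulation on its destructible and a Destroy call at its own location.
; Any overlap switches the Box's overlap events off after a short delay; without an overlap they stay on.
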(event `InputAction|Img_Attack`
  (params (Key :type "Key Structure"))
  (:`Pressed`
    (set `PrimitiveComponent.bGenerateOverlapEvents` true (`self.Box`))))

(event `self.Box.OnComponentBeginOverlap`
  (params (OverlappedComponent :type "PrimitiveComponent Object Reference") (OtherActor :type "Actor Object Reference") (OtherComp :type "PrimitiveComponent Object Reference") (OtherBodyIndex :type Integer) (bFromSweep :type Boolean) (SweepResult :type "HitResult Structure (by ref)"))
  (bind _box (`self.Box`))
  (bind `_as段ボール_dm` (cast `/Game/Blueprint/gimmick/破壊可能オブジェクト/段ボール_DM` OtherActor)
    (:`then`
      (`PrimitiveComponent.SetSimulatePhysics` (`/Game/Blueprint/gimmick/破壊可能オブジェクト/段ボール_DM.Destructible` `_as段ボール_dm`) true)
      (`self.Destroy` `_as段ボール_dm` (`self.K2_GetActorLocation` OtherActor))
      (`KismetSystemLibrary.Delay` 1.0)
      (set `PrimitiveComponent.bGenerateOverlapEvents` false _box))
    (:`CastFailed`
      (`KismetSystemLibrary.Delay` 1.0)
      (set `PrimitiveComponent.bGenerateOverlapEvents` false _box))))

(fn `UserConstructionScript`
  (`parent.UserConstructionScript`))