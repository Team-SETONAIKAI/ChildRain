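; Parent (親) Blueprint for the Imaginary Friend pawn, providing player movement and camera control in what appears to be a side-view setup.
; The MoveRight axis adds movement along a forward vector built from only the control rotation's pitch, with yaw and roll zeroed.
; Two CameraRotation axes apply raw yaw and pitch offsets to the side-view camera component's relative rotation, without clamping or delta-time scaling.
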(event `InputAxis|MoveRight`
  (params (AxisValue :type "Float (single-precision)"))
  (`self.AddMovementInput` (`KismetMathLibrary.GetForwardVector` (`KismetMathLibrary.MakeRotator` 0.0 (.pitch (`self.GetControlRotation`)))) AxisValue))

(event `InputAxis|CameraRotation_X`
  (params (AxisValue :type "Float (single-precision)"))
  (`SceneComponent.K2_AddRelativeRotation` (`self.SIdeViweCamera`) (`KismetMathLibrary.MakeRotator` 0.0 0.0 AxisValue) false false))

(event `InputAxis|CameraRotation_Y`
  (params (AxisValue :type "Float (single-precision)"))
  (`SceneComponent.K2_AddRelativeRotation` (`self.SIdeViweCamera`) (`KismetMathLibrary.MakeRotator` 0.0 AxisValue) false false))

(fn `UserConstructionScript`)