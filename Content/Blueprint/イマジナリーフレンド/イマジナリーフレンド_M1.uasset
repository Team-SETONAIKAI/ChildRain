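; Imaginary-friend actor (イマジナリーフレンド_M1) that damages enemies through an attack hit box.
; The Jump input toggles an attack flag and prints a battle cry when it arms.
; When the hit box begins overlapping an Enemy_親Class actor while armed, it applies fixed damage and clears the flag.
; The enemy itself is passed as the damage causer.
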(event `InputAction|Jump`
  (params (Key :type "Key Structure"))
  (:`Pressed`
    (if (`self.Atack_Flg`)
      (set `self.Atack_Flg` false)
      (else
        (set `self.Atack_Flg` true)
        (`KismetSystemLibrary.PrintString` "くらえ！")))))

(event `self.Box(AtackHIt).OnComponentBeginOverlap`
  (params (OverlappedComponent :type "PrimitiveComponent Object Reference") (OtherActor :type "Actor Object Reference") (OtherComp :type "PrimitiveComponent Object Reference") (OtherBodyIndex :type Integer) (bFromSweep :type Boolean) (SweepResult :type "HitResult Structure (by ref)"))
  (bind `_asenemy_親class` (cast `/Game/Blueprint/Enemy/Enemy_親Class` OtherActor))
  (if (`self.Atack_Flg`)
    (`GameplayStatics.ApplyDamage` `_asenemy_親class` 20.0 null OtherActor)
    (set `self.Atack_Flg` false)))

(fn `UserConstructionScript`
  (`parent.UserConstructionScript`))