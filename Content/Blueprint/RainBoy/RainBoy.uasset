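; RainBoy is the side-view player character, with movement, limited multi-jump, crouch and health.
; One vertical axis picks crouch, stand or jump, with LockButton blocking held-input repeats.
; Moving or rotating the camera line-traces for puddles, letting X set summon flags for an imaginary friend, while A sets transform flags.
; At zero health it shows a fading GameOver widget and slides the spring arm along negative X each tick.
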(event `InputAxis|MoveRight`
  (params (AxisValue :type "Float (single-precision)"))
  ;[1 1 1] 移動処理
  (if (`self.Alive`)
    (if (not (`self.LockButton`))
      (set `self.RunButton` AxisValue)
      (`self.AddMovementInput` (`KismetMathLibrary.GetForwardVector` (`KismetMathLibrary.MakeRotator` 0.0 (.pitch (`self.GetControlRotation`)))) AxisValue)
      (`self.Hit Camera Puddle`))))

(event `self.ReceiveAnyDamage`
  (params (Damage :type "Float (single-precision)") (DamageType :type "DamageType Object Reference") (InstigatedBy :type "Controller Object Reference") (DamageCauser :type "Actor Object Reference"))
  ;[1 1 1] ダメージ処理
  (bind _output_get (set `self.Helth` (- (`self.Helth`) Damage)))
  (if (<= _output_get 0.0)
    (set `self.Alive` false)
    (bind _returnvalue (`|CreateWidget` "/Game/UI/プレイ中/GameOver.GameOver_C"))
    (`UserWidget.AddToViewport` _returnvalue 0)
    (`UserWidget.PlayAnimation` _returnvalue (`/Game/UI/プレイ中/GameOver.FadeOutAnim` _returnvalue) 0.0 1 "Forward" 1.0 false)
    (`KismetSystemLibrary.PrintString` "Guhu")))

(event `InputAxis|MoveTop`
  (params (AxisValue :type "Float (single-precision)"))
  (if (`self.Alive`)
    ;[1 1 1] ボタンが押されてる？
    (if (!= AxisValue 0.0)
      ;[1 1 1] ボタンを一度離していない？
      (if (!= (`self.LockButton`) true)
        (bind _setint (`self.Check_TopButton` AxisValue))
        (switch `int` _setint
          (:`0`
            (`self.SquatOn`))
          (:`1`
            (`self.SquatOff`))
          (:`2`
            (`self.Custom_Jump`))))
      (else
        (set `self.LockButton` false)))))

(event `Custom_Jump`
  ;[1 1 1] Jump処理
  (bind _counter (`/Engine/EditorBlueprintResources/StandardMacros.Do N` (`self.JumpMaxCount`) :!label _label)
    (:`Exit`
      (switch `int` _counter
        (:`1`
          _)
        (:`2`
          _))
      (set `self.GetOnLanded` false)
      (`self.Jump`))))

(event `self.OnLanded`
  (params (Hit :type "HitResult Structure (by ref)"))
  ;[1 1 1] Jump処理
  (set `self.GetOnLanded` true)
  (goto _label :!via `Reset`))

(event `self.ReceiveTick`
  (params (DeltaSeconds :type "Float (single-precision)"))
  (bind _springarm (`self.SpringArm`))
  (if (not (`self.Alive`))
    (`SceneComponent.K2_SetWorldLocation` _springarm (- (`SceneComponent.K2_GetComponentLocation` _springarm) (1.0 0.0 0.0)) false false)))

(event `InputAxis|CameraRotation_X`
  (params (AxisValue :type "Float (single-precision)"))
  ;[1 1 1] カメラ操作_当たり判定
  (`SceneComponent.K2_AddRelativeRotation` (`self.Side View Camera`) (`KismetMathLibrary.MakeRotator` 0.0 0.0 AxisValue) false false)
  (`self.Hit Camera Puddle` :!label _label_2))

(event `InputAxis|CameraRotation_Y`
  (params (AxisValue :type "Float (single-precision)"))
  ;[1 1 1] カメラ操作_当たり判定
  (`SceneComponent.K2_AddRelativeRotation` (`self.Side View Camera`) (`KismetMathLibrary.MakeRotator` 0.0 AxisValue) false false)
  (goto _label_2))

(event `InputAction|XButton_Action`
  (params (Key :type "Key Structure"))
  ;[1 1 1] XButton_Action
  (:`Pressed`
    (if (`self.Alive`)
      (if (`self.HitWater`)
        ;[1 1 1] イマジナリーフレンド召喚
        (if (`self.CreateMode`)
          (`KismetSystemLibrary.PrintString` "CreateMode = true!")
          (else
            (bind _output_get (set `self.CreateOrChenge_ImgFriend` 1))
            (`KismetSystemLibrary.PrintString` (`KismetStringLibrary.Conv_IntToString` _output_get))
            (set `self.CreateMode` true)
            (`KismetSystemLibrary.PrintString` "セット完了！")))))))

(event `InputAction|AButton_Special`
  (params (Key :type "Key Structure"))
  ;[1 1 1] AButton_Special
  (:`Pressed`
    (if (`self.Alive`)
      ;[1 1 1] イマジナリーフレンド変身
      (if (`self.CreateMode`)
        (`KismetSystemLibrary.PrintString` "イマジナリーフレンド生成中！")
        (elif (!= (`self.CreateOrChenge_ImgFriend`) 0)
          (`KismetSystemLibrary.PrintString` "イマジナリーフレンド変身中！")
          (else
            (set `self.Chenge_ImgFriendMode` true)
            (if (== (`self.Chenge_ImgFriendNo`) 0)
              (set `self.Chenge_ImgFriendNo` 1)
              (else
                (set `self.Chenge_ImgFriendNo` 0)))
            (set `self.CreateOrChenge_ImgFriend` 2)
            (set `self.CreateMode` true)
            (`KismetSystemLibrary.PrintString` "イマジナリーフレンド変身開始！")))))))

(fn `Check_TopButton`
  (params (AxisValue :type "Float (double-precision)"))
  (returns (SetInt :type Integer))
  (bind _output_get (set `self.AxisValue` AxisValue))
  ;[1 1 1] 下に押された？
  (if (== _output_get -1.0)
    ;[1 1 1] 既にしゃがんでる?
    (if (== (`self.SquatButton`) -1.0)
      (return 999)
      (elif (`self.GetOnLanded`)
        (return 0)))
    (else
      ;[1 1 1] 上に押された？
      (if (== (`self.AxisValue`) 1.0)
        ;[1 1 1] 既にしゃがんでる?
        (if (== (`self.SquatButton`) -1.0)
          (return 1)
          (else
            (return 2)))
        (else
          (`KismetSystemLibrary.PrintString` "何事!?")
          (return 999))))))

(fn `Hit Camera Puddle`
  (bind _side_view_camera (`self.Side View Camera`))
  (bind _returnvalue (`SceneComponent.K2_GetComponentLocation` _side_view_camera))
  (bind (_outhit _returnvalue_2) (`KismetSystemLibrary.LineTraceSingle` :`Start` _returnvalue :`End` (+ _returnvalue (* (`SceneComponent.GetForwardVector` _side_view_camera) 1000.0)) :`TraceChannel` "TraceTypeQuery3" :`DrawDebugType` "ForOneFrame"))
  (if _returnvalue_2
    (set `self.Puddle_Transform` (`self.GetTransform` (`.HitActor` (`GameplayStatics.BreakHitResult` _outhit))))
    (set `self.HitWater` true)
    (return)
    (else
      (set `self.HitWater` false)
      (return))))

(fn `SquatOff`
  (`CapsuleComponent.SetCapsuleHalfHeight` (`self.CapsuleComponent`) 64.0 true)
  (`SceneComponent.K2_SetRelativeTransform` (`self.Mesh`) (`KismetMathLibrary.MakeTransform` (`KismetMathLibrary.MakeVector` (.x (.location (`SceneComponent.GetRelativeTransform` (`self.Mesh`)))) (.y (.location (`SceneComponent.GetRelativeTransform` (`self.Mesh`)))) -65.0) (.rotation (`SceneComponent.GetRelativeTransform` (`self.Mesh`))) (.scale (`SceneComponent.GetRelativeTransform` (`self.Mesh`)))) false false)
  (set `self.SquatButton` 0.0)
  (set `self.LockButton` true)
  (return))

(fn `SquatOn`
  (`CapsuleComponent.SetCapsuleHalfHeight` (`self.CapsuleComponent`) 44.0 true)
  (`SceneComponent.K2_SetRelativeTransform` (`self.Mesh`) (`KismetMathLibrary.MakeTransform` (`KismetMathLibrary.MakeVector` 0.0 0.0 -45.0) (.rotation (`SceneComponent.GetRelativeTransform` (`self.Mesh`))) (.scale (`SceneComponent.GetRelativeTransform` (`self.Mesh`)))) false false)
  (set `self.SquatButton` -1.0)
  (set `self.LockButton` true)
  (return))

(fn `UserConstructionScript`)